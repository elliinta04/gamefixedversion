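; Conveyor belt actor that pushes actors along its surface and is also set up to travel between two points.
; Each tick, it offsets every actor overlapping its Box along the Arrow's forward vector, scaled by Speed and delta time, without sweeping for collision.
; The construction script gives the InterpToMovement component two relative control points, the origin and Movetopos, as the belt's own path.
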(event `self.ReceiveTick`
  (params (DeltaSeconds :type "Float (single-precision)"))
  (for _array_element (`PrimitiveComponent.GetOverlappingActors` (`self.Box`) null)
    (`self.K2_AddActorWorldOffset` _array_element (* (`KismetMathLibrary.GetForwardVector` (`SceneComponent.K2_GetComponentRotation` (`self.Arrow`))) (* DeltaSeconds (`self.speed`))) false false)))

(fn `UserConstructionScript`
  (`InterpToMovementComponent.AddControlPointPosition` (`self.InterpToMovement`) (0.0 0.0 0.0) true)
  (`InterpToMovementComponent.AddControlPointPosition` (`self.InterpToMovement`) (`self.movetopos`) true))