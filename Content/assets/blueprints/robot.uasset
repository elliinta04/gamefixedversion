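; Robot actor that moves along a referenced spline actor's path from the moment play begins.
; A timeline, with play rate scaled by TimeToComplete, lerps distance from zero to the spline length and sets world location and rotation from the spline each update.
; The construction script applies the configurable ObjectMesh to its static mesh.
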(event `self.ReceiveBeginPlay`
  (`self.moveobjrct`))

(event `moveobjrct`
  (bind _spline (`/Game/assets/blueprints/splineplease.Spline` (`self.splinetofollow`)))
  (`TimelineComponent.SetPlayRate` (`self.T_move`) (/ 1.0 (`self.time to complete`)))
  (bind (_direction _moverack) (`Timeline|T_move`)
    (:`Update`
      (bind _returnvalue (`KismetMathLibrary.Lerp` 0.0 (`SplineComponent.GetSplineLength` _spline) _moverack))
      (`self.K2_SetActorLocationAndRotation` (`SplineComponent.GetLocationAtDistanceAlongSpline` _spline _returnvalue "World") (`SplineComponent.GetRotationAtDistanceAlongSpline` _spline _returnvalue "World")))))

(fn `UserConstructionScript`
  (`StaticMeshComponent.SetStaticMesh` (`self.robot`) (`self.object mesh`)))