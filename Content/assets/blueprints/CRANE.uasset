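; Crane actor that moves its skeletal mesh along a spline as a hazard for characters.
; Tick advances distance at a set speed and applies the spline transform with height and yaw offsets, restarting at the end when looping is enabled.
; Box overlap launches characters; Hit calls ApplyDamage before casting to the third-person character, then spawns short-lived sparks once.
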(event `self.ReceiveTick`
  (params (DeltaSeconds :type "Float (single-precision)"))
  (bind _returnvalue (`SplineComponent.GetTransformAtDistanceAlongSpline` (`self.Spline`) (`self.DISTANCE ALONG SPLINE`) "Local" false))
  (set `self.DISTANCE ALONG SPLINE` (+ (* DeltaSeconds (`self.SPLINE SPEED`)) (`self.DISTANCE ALONG SPLINE`)))
  (`SceneComponent.K2_SetRelativeTransform` (`self.SkeletalMesh`) (`KismetMathLibrary.MakeTransform` (`KismetMathLibrary.MakeVector` (.x (.location _returnvalue)) (.y (.location _returnvalue)) (+ (.z (.location _returnvalue)) -89.0)) (`KismetMathLibrary.MakeRotator` (.roll (.rotation _returnvalue)) (.pitch (.rotation _returnvalue)) (+ (.yaw (.rotation _returnvalue)) -90.0)) (`SceneComponent.RelativeScale3D` (`self.SkeletalMesh`))) false false)
  (if (`self.LOOP`)
    (if (> (`self.DISTANCE ALONG SPLINE`) (`SplineComponent.GetSplineLength` (`self.Spline`)))
      (set `self.DISTANCE ALONG SPLINE` 0.0))))

(event `self.Box.OnComponentBeginOverlap`
  (params (OverlappedComponent :type "PrimitiveComponent Object Reference") (OtherActor :type "Actor Object Reference") (OtherComp :type "PrimitiveComponent Object Reference") (OtherBodyIndex :type Integer) (bFromSweep :type Boolean) (SweepResult :type "HitResult Structure (by ref)"))
  (bind _ascharacter (cast `Character` OtherActor))
  (`Character.LaunchCharacter` _ascharacter (150.0 150.0 150.0) false false))

(event `self.ReceiveHit`
  (params (MyComp :type "PrimitiveComponent Object Reference") (Other :type "Actor Object Reference") (OtherComp :type "PrimitiveComponent Object Reference") (bSelfMoved :type Boolean) (HitLocation :type "Vector Structure") (HitNormal :type "Vector Structure") (NormalImpulse :type "Vector Structure") (Hit :type "HitResult Structure (by ref)"))
  (`GameplayStatics.ApplyDamage` (stale _asbp_third_person_character) 10.0)
  (bind _asbp_third_person_character (cast `/Game/ThirdPerson/Blueprints/BP_ThirdPersonCharacter` Other))
  (`/Engine/EditorBlueprintResources/StandardMacros.DoOnce` false
    (:`Completed`
      (bind _returnvalue (`GameplayStatics.SpawnEmitterAtLocation` "/Game/StarterContent/Particles/P_Sparks.P_Sparks" (`self.K2_GetActorLocation` _asbp_third_person_character)))
      (`KismetSystemLibrary.Delay` 1.0)
      (`ActorComponent.K2_DestroyComponent` _returnvalue))))

(fn `UserConstructionScript`)